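; BP_ChangeColor is an interactable puzzle piece whose cube cycles from red to green to blue and back on each interaction.
; SwitchColor maps the color state to a vector and sets it on the cube's Color material parameter, with the construction script initializing it to red.
; After each change, it sends its index and new color to the referenced door through TestSolveMessage.
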(event EventInteraction
  (bind _output_get (Variables|Default|SetColorState (Utilities|Select :Index (Variables|Default|GetColorState) :NewEnumerator0 "NewEnumerator1" :NewEnumerator1 "NewEnumerator2" :NewEnumerator2 "NewEnumerator0")))
  (CallFunction|SwitchColor _output_get)
  (Class|BPIInteract|TestSolve(Message) (Variables|Default|GetDoorRef) (Variables|Default|GetIndex) (Variables|Default|GetColorState)))

(fn ConstructionScript
  (CallFunction|SwitchColor "NewEnumerator0"))

(fn SwitchColor
  (params (CurrentColor :type ECubeColor%20Enum :default "NewEnumerator0"))
  (Rendering|Material|SetVectorParameterValueonMaterials (Variables|Default|GetCube) "Color" (Utilities|Select :Index CurrentColor :NewEnumerator0 "1.000000,0.000000,0.000000" :NewEnumerator1 "0.000000,1.000000,0.000000" :NewEnumerator2 "0.000000,0.000000,1.000000")))