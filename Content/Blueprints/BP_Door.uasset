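; Door that swings open or closed, doubling as the outcome of a color-combination puzzle.
; BeginPlay fills the Solution array with random picks from three enum values; TestSolve updates CurrentColors and triggers the door when the arrays match.
; Interaction and a solved match share a FlipFlop that plays or reverses a yaw Timeline scaled by AngleRotation.
; The code binding Interaction to BP_Player is disconnected.
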(event EventBeginPlay
  (bind _solution (Variables|Default|GetSolution))
  (for (_ _array_index) _solution
    (Utilities|Array|SetArrayElem _solution _array_index (Utilities|Select :Index (Math|Random|RandomIntegerinRange 0 2) :Option%200 "NewEnumerator0" :Option%201 "NewEnumerator1" :Option%202 "NewEnumerator2"))))

(event Collision|EventActorBeginOverlap
  (params (OtherActor :type Actor%20Object%20Reference)))

(event EventTick
  (params (DeltaSeconds :type Float%20%28single-precision%29)))

(event EventInteraction
  (Utilities|FlowControl|FlipFlop
    (:A
      (bind _newtrack_0 (Timeline|Timeline Play)
        (:Update
          (Transformation|SetRelativeRotation (Variables|Default|GetStaticMesh) (Math|Rotator|MakeRotator 0.0 0.0 (* _newtrack_0 (Variables|Default|GetAngleRotation))) false false))))
    (:B
      (Timeline|Timeline Reverse))))

(event EventTestSolve
  (params (Index :type Integer) (NewColor :type ECubeColor%20Enum :default "NewEnumerator0"))
  (Utilities|Array|SetArrayElem (Variables|Default|GetCurrentColors) Index NewColor)
  (if (Utilities|Array|Identical (Variables|Default|GetSolution) (Variables|Default|GetCurrentColors))
    (Utilities|FlowControl|FlipFlop
      (:A
        (bind _newtrack_0 (Timeline|Timeline Play)
          (:Update
            (Transformation|SetRelativeRotation (Variables|Default|GetStaticMesh) (Math|Rotator|MakeRotator 0.0 0.0 (* _newtrack_0 (Variables|Default|GetAngleRotation))) false false))))
      (:B
        (Timeline|Timeline Reverse)))))

(fn ConstructionScript)